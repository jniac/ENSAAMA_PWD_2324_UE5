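; Elevator Blueprint that raises its platform component while another actor overlaps it.
; Begin and end overlap events set a ShouldGoUp flag with no filter on the overlapping actor.
; While the flag is set, Tick increases the height at a constant frame-rate-independent speed, clamped to LimitZ, and applies it as the platform's relative Z.
; Ending the overlap halts the platform in place, as no logic lowers it.
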(event `self.ReceiveActorEndOverlap`
  (params (OtherActor :type "Actor Object Reference"))
  (set `self.shouldGoUp` false))

(event `self.ReceiveBeginPlay`)

(event `self.ReceiveActorBeginOverlap`
  (params (OtherActor :type "Actor Object Reference"))
  (set `self.shouldGoUp` true))

(event `self.ReceiveTick`
  (params (DeltaSeconds :type "Float (single-precision)"))
  (if (`self.shouldGoUp`)
    (bind _output_get (set `self.up` (`KismetMathLibrary.FClamp` (+ (`self.up`) (* DeltaSeconds 100.0)) 0.0 (`self.limitZ`))))
    (`SceneComponent.K2_SetRelativeLocation` (`self.Plateforme`) (`KismetMathLibrary.MakeVector` 0.0 0.0 _output_get) false false)))

(fn `UserConstructionScript`)