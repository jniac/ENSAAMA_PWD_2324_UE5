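; Elevator actor that moves a platform in a straight line between its local origin and a destination marked by the Sphere component.
; An actor overlap near either end of the travel sets Direction toward the opposite end.
; Tick advances a clamped Alpha, scaled by Velocity over the distance for constant speed, then lerps the platform's relative location.
; The construction script runs the same platform update to show its position for the current Alpha.
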(event `self.ReceiveBeginPlay`)

(event `self.ReceiveActorBeginOverlap`
  (params (OtherActor :type "Actor Object Reference"))
  (if (or (< (`self.Alpha`) 0.1) (> (`self.Alpha`) 0.9))
    (set `self.Direction` (< (`self.Alpha`) 0.5))))

(event `self.ReceiveActorEndOverlap`
  (params (OtherActor :type "Actor Object Reference")))

(event `self.ReceiveTick`
  (params (DeltaSeconds :type "Float (single-precision)"))
  (`self.Update Alpha` DeltaSeconds)
  (`self.Update Platform`))

(fn `Update Alpha`
  (params (deltaSeconds :type "Float (double-precision)"))
  (set `self.Alpha` (`KismetMathLibrary.FClamp` (+ (`self.Alpha`) (* (/ deltaSeconds (/ (`KismetMathLibrary.VSize` (`SceneComponent.RelativeLocation` (`self.Sphere`))) (`self.Velocity`))) (`KismetMathLibrary.SelectFloat` 1.0 -1.0 (`self.Direction`)))))))

(fn `Update Platform`
  (`SceneComponent.K2_SetRelativeLocation` (`self.Plateforme`) (`KismetMathLibrary.VLerp` (`KismetMathLibrary.MakeVector` 0.0) (`SceneComponent.RelativeLocation` (`self.Sphere`)) (`self.Alpha`)) false false))

(fn `UserConstructionScript`
  (`self.Update Platform`))