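; Flower actor that blooms when a Character overlaps it, rotating three rings of petals while a light brightens and spores activate.
; One Timeline drives the petal rings on separate curves, each lerping roll while keeping pitch and yaw.
; Its LightValue curve sets the light intensity and switches the Niagara spores on above a small threshold.
; The construction script resets all petals to their starting pose.
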(event `self.ReceiveActorBeginOverlap`
  (params (OtherActor :type "Actor Object Reference"))
  (cast `Character` OtherActor)
  (bind (_direction _timea _timeb _timec _lightvalue) (`Timeline|Timeline`)
    (:`Update`
      (`self.UpdatePetalsA` _timea)
      (`self.UpdatePetalsB` _timeb)
      (`LightComponent.SetIntensity` (`self.g`) (`KismetMathLibrary.Lerp` 500.0 25000.0 _lightvalue))
      (`self.UpdtaePetalsC` _timec)
      (`ActorComponent.SetActive` (`self.rse_Ni_Spores`) (> _lightvalue 0.1) false))))

(fn `UpdatePetalsA`
  (params (TimeA :type "Float (double-precision)"))
  (set `self.timeA` TimeA)
  (for _array_element (`|MakeArray` (`self.rse_SM_PetalDeFou`) (`self.rse_SM_PetalDeFou1`) (`self.rse_SM_PetalDeFou2`) (`self.rse_SM_PetalDeFou3`))
    (bind (_relativerotation_roll _relativerotation_pitch _relativerotation_yaw) (`KismetMathLibrary.BreakRotator` (`SceneComponent.RelativeRotation` _array_element)))
    (`SceneComponent.K2_SetRelativeRotation` _array_element (`KismetMathLibrary.MakeRotator` (`KismetMathLibrary.Lerp` 60.0 10.0 (`self.timeA`)) _relativerotation_pitch _relativerotation_yaw) false false)))

(fn `UpdatePetalsB`
  (params (TimeB :type "Float (double-precision)"))
  (set `self.timeB` TimeB)
  (for _array_element (`|MakeArray` (`self.rse_SM_PetalDeFou4`) (`self.rse_SM_PetalDeFou5`) (`self.rse_SM_PetalDeFou6`) (`self.rse_SM_PetalDeFou7`))
    (bind (_relativerotation_roll _relativerotation_pitch _relativerotation_yaw) (`KismetMathLibrary.BreakRotator` (`SceneComponent.RelativeRotation` _array_element)))
    (`SceneComponent.K2_SetRelativeRotation` _array_element (`KismetMathLibrary.MakeRotator` (`KismetMathLibrary.Lerp` 50.0 10.0 (`self.timeB`)) _relativerotation_pitch _relativerotation_yaw) false false)))

(fn `UpdtaePetalsC`
  (params (TimeC :type "Float (double-precision)"))
  (set `self.timeC` TimeC)
  (for _array_element (`|MakeArray` (`self.rse_SM_Petal_C`) (`self.rse_SM_Petal_C1`) (`self.rse_SM_Petal_C2`) (`self.rse_SM_Petal_C3`) (`self.rse_SM_Petal_C4`) (`self.rse_SM_Petal_C5`))
    (bind (_relativerotation_roll _relativerotation_pitch _relativerotation_yaw) (`KismetMathLibrary.BreakRotator` (`SceneComponent.RelativeRotation` _array_element)))
    (`SceneComponent.K2_SetRelativeRotation` _array_element (`KismetMathLibrary.MakeRotator` (`KismetMathLibrary.Lerp` 40.0 5.0 (`self.timeC`)) _relativerotation_pitch _relativerotation_yaw) false false)))

(fn `UserConstructionScript`
  (`self.UpdatePetalsA` 0.0)
  (`self.UpdatePetalsB` 0.0)
  (`self.UpdtaePetalsC` 0.0))