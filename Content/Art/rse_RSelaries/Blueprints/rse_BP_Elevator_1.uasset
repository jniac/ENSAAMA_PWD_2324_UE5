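; Elevator actor whose platform travels diagonally up and along negative local Y while an actor overlaps it.
; Begin and end overlap events toggle a ShouldGo flag without filtering which actor triggered them.
; Tick advances or retracts the platform's relative Y and Z offsets at constant frame-rate-independent speeds, clamped to LimitY and LimitZ, with the return running twice as fast.
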(event `self.ReceiveActorEndOverlap`
  (params (OtherActor :type "Actor Object Reference"))
  (set `self.shouldGo` false))

(event `self.ReceiveBeginPlay`)

(event `self.ReceiveActorBeginOverlap`
  (params (OtherActor :type "Actor Object Reference"))
  (set `self.shouldGo` true))

(event `self.ReceiveTick`
  (params (DeltaSeconds :type "Float (single-precision)"))
  (bind _returnvalue (* DeltaSeconds -400.0))
  (bind _returnvalue_2 (* DeltaSeconds 180.0))
  (if (`self.shouldGo`)
    (set `self.up` (`KismetMathLibrary.FClamp` (+ (`self.up`) _returnvalue_2) 0.0 (`self.limitZ`)))
    (set `self.forward` (`KismetMathLibrary.FClamp` (+ _returnvalue (`self.forward`)) (`self.limitY`) 0.0))
    (else
      (set `self.up` (`KismetMathLibrary.FClamp` (+ (* _returnvalue_2 -2.0) (`self.up`)) 0.0 (`self.limitZ`)))
      (set `self.forward` (`KismetMathLibrary.FClamp` (+ (* _returnvalue -2.0) (`self.forward`)) (`self.limitY`) 0.0))))
  (`SceneComponent.K2_SetRelativeLocation` (`self.Plateforme`) (`KismetMathLibrary.MakeVector` 0.0 (`self.forward`) (`self.up`)) false false))

(fn `UserConstructionScript`)